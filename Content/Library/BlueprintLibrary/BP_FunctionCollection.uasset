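; Actor-based collection of procedural geometry helpers for modular mesh, polygon and spline construction, with empty events and construction script.
; Samplers split edges and splines into whole units, stretched or respaced to fit, and spawners add static or spline mesh components.
; Polygons shrink along corner bisectors, then become extruded dynamic meshes.
; Other helpers offset splines, find crossings by distance marching and build box corners; PolygonPartitioningA is unfinished, returning zero cut points.
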(fn `Average`
  (params (Whole :type "Float (double-precision)") (Unit :type "Float (double-precision)"))
  (returns (Long :type "Float (double-precision)") (Count :type Integer))
  (bind (_remainder _returnvalue) (`KismetMathLibrary.FMod` Whole Unit))
  (bind _returnvalue_2 (`KismetMathLibrary.Max` (`KismetMathLibrary.SelectInt` (+ _returnvalue 1) _returnvalue (> _remainder (/ Unit 2.0))) 1))
  (return (/ Whole _returnvalue_2) _returnvalue_2))

(fn `Create Box Corner`
  (params (BaseTransform :type "Transform Structure (by ref)") (Width :type "Float (double-precision)") (Long :type "Float (double-precision)"))
  (returns (PointArray :type "Array of Transform Structure"))
  (locals (PointArray_Var :type "Array of Transform Structure"))
  (bind _location (.location BaseTransform))
  (bind _rotation (.rotation BaseTransform))
  (bind _pointarray_var (`local.PointArray_Var`))
  (bind _returnvalue (* (`KismetMathLibrary.GetRightVector` _rotation) (/ Long 2.0)))
  (bind _returnvalue_2 (* (`KismetMathLibrary.GetForwardVector` _rotation) (/ Width 2.0)))
  (bind _returnvalue_3 (* _returnvalue_2 (-1.0 -1.0 -1.0)))
  (bind _returnvalue_4 (* _returnvalue (-1.0 -1.0 -1.0)))
  (`KismetArrayLibrary.Array_AddUnique` _pointarray_var (`KismetMathLibrary.MakeTransform` (+ _location (+ _returnvalue_2 _returnvalue))))
  (`KismetArrayLibrary.Array_AddUnique` _pointarray_var (`KismetMathLibrary.MakeTransform` (+ _location (+ _returnvalue_2 _returnvalue_4))))
  (`KismetArrayLibrary.Array_AddUnique` _pointarray_var (`KismetMathLibrary.MakeTransform` (+ _location (+ _returnvalue_3 _returnvalue_4))))
  (`KismetArrayLibrary.Array_AddUnique` _pointarray_var (`KismetMathLibrary.MakeTransform` (+ _location (+ _returnvalue_3 _returnvalue))))
  (return (`local.PointArray_Var`)))

(fn `EdgeSampler`
  (params (BeginLocation :type "Vector Structure") (EndLocation :type "Vector Structure") (Unit_Mesh :type "StaticMesh Object Reference"))
  (returns (PointArray :type "Array of Transform Structure"))
  (locals (PointArray_Var :type "Array of Transform Structure"))
  (bind (_long _width _height _alongx) (`self.GetMeshSize` Unit_Mesh))
  (bind (_returnvalue_roll _returnvalue_pitch _returnvalue_yaw) (`KismetMathLibrary.BreakRotator` (`KismetMathLibrary.FindLookAtRotation` BeginLocation EndLocation)))
  (bind (_remainder _returnvalue) (`KismetMathLibrary.FMod` (`KismetMathLibrary.Vector_Distance` BeginLocation EndLocation) _long))
  (bind _returnvalue_2 (<= _remainder (/ _long 2.0)))
  (bind _returnvalue_3 (`KismetMathLibrary.SelectInt` _returnvalue (+ _returnvalue 1) _returnvalue_2))
  (bind _returnvalue_4 (`KismetMathLibrary.Max` _returnvalue_3 1))
  (bind _returnvalue_5 (and (>= _returnvalue_3 1) _returnvalue_2))
  (bind _returnvalue_6 (- _long (/ (- _long _remainder) _returnvalue_4)))
  (bind _returnvalue_7 (+ _long (/ _remainder _returnvalue_4)))
  (bind _returnvalue_8 (`KismetMathLibrary.SelectFloat` (/ _returnvalue_7 _long) (/ _returnvalue_6 _long) _returnvalue_5))
  (`KismetArrayLibrary.Array_Clear` (`local.PointArray_Var`))
  (for _index (range _returnvalue_4)
    (`KismetArrayLibrary.Array_Add` (`local.PointArray_Var`) (`KismetMathLibrary.MakeTransform` (+ (* (* _index (`KismetMathLibrary.SelectFloat` _returnvalue_7 _returnvalue_6 _returnvalue_5)) (`KismetMathLibrary.Normal` (- EndLocation BeginLocation) 0.0)) BeginLocation) (`KismetMathLibrary.MakeRotator` _returnvalue_roll _returnvalue_pitch (+ _returnvalue_yaw (`KismetMathLibrary.SelectFloat` 0.0 90.0 _alongx))) (`KismetMathLibrary.SelectVector` (`KismetMathLibrary.MakeVector` _returnvalue_8 1.0 1.0) (`KismetMathLibrary.MakeVector` 1.0 _returnvalue_8 1.0) _alongx))))
  (return (`local.PointArray_Var`)))

(fn `FindSplineCrossPoint`
  (params (SplineA :type "SplineComponent Object Reference") (SplineB :type "SplineComponent Object Reference"))
  (returns (CrossLocation :type "Vector Structure") (HaveCross :type Boolean))
  (locals (MinDistance :type "Float (double-precision)" :default 1e+16) (SampleDistance :type "Float (double-precision)"))
  (bind _splineb (`local.SplineB`))
  (bind _returnvalue (`SplineComponent.GetLocationAtDistanceAlongSpline` (`local.SplineA`) (`local.SampleDistance`) "World"))
  (bind _returnvalue_2 (`KismetMathLibrary.Vector_Distance` (`SplineComponent.GetLocationAtDistanceAlongSpline` _splineb (`SplineComponent.GetDistanceAlongSplineAtLocation` _splineb _returnvalue "World") "World") _returnvalue))
  (while (and (> (`local.MinDistance`) 15.0) (not (> (`local.SampleDistance`) (`SplineComponent.GetSplineLength` (`local.SplineA`)))))
    (set `local.MinDistance` _returnvalue_2)
    (set `local.SampleDistance` (+ _returnvalue_2 (`local.SampleDistance`))))
  (return (`SplineComponent.GetLocationAtDistanceAlongSpline` (`local.SplineA`) (`local.SampleDistance`) "World") (not (> (`local.MinDistance`) 15.0))))

(fn `GetBisectorVector`
  (params (A :type "Vector Structure") (B :type "Vector Structure") (C :type "Vector Structure"))
  (returns (BisectorVector :type "Vector Structure"))
  (return (`KismetMathLibrary.Normal` (+ (`KismetMathLibrary.Normal` (- A B)) (`KismetMathLibrary.Normal` (- C B))))))

(fn `GetLongestEdge`
  (params (CornerArray :type "Array of Vector Structure"))
  (returns (LongestEdge_Index :type Integer))
  (locals (EdgeLong :type "Float (double-precision)") (PointIndex :type Integer))
  (for (_ _array_index) CornerArray
    (bind (_lastpointlocation _currentpointlocation _nextpointlocation) (`self.GetNearPoints` CornerArray _array_index))
    (bind _returnvalue (`KismetMathLibrary.Vector_Distance` _currentpointlocation _nextpointlocation))
    (if (> _returnvalue (`local.EdgeLong`))
      (set `local.EdgeLong` _returnvalue)
      (set `local.PointIndex` _array_index)))
  (return (`local.PointIndex`)))

(fn `GetMeshSize`
  (params (Mesh :type "StaticMesh Object Reference"))
  (returns (Long :type "Float (double-precision)") (Width :type "Float (double-precision)") (Height :type "Float (double-precision)") (AlongX :type Boolean))
  (bind (_min _max) (break `Box` (`StaticMesh.GetBoundingBox` Mesh)))
  (bind (_returnvalue_x _returnvalue_y _returnvalue_z) (`KismetMathLibrary.BreakVector` (- _min _max)))
  (bind _returnvalue (`KismetMathLibrary.Abs` _returnvalue_y))
  (bind _returnvalue_2 (`KismetMathLibrary.Abs` _returnvalue_x))
  (return (`KismetMathLibrary.FMax` _returnvalue_2 _returnvalue) (`KismetMathLibrary.FMin` _returnvalue_2 _returnvalue) (`KismetMathLibrary.Abs` _returnvalue_z) (> _returnvalue_2 _returnvalue)))

(fn `GetNearPoints`
  (params (PointArray :type "Array of Vector Structure (by ref)") (PointIndex :type Integer))
  (returns (LastPointLocation :type "Vector Structure") (CurrentPointLocation :type "Vector Structure") (NextPointLocation :type "Vector Structure"))
  (bind _returnvalue (`KismetArrayLibrary.Array_LastIndex` PointArray))
  (return (`KismetMathLibrary.SelectVector` (`|GetArrayItem` PointArray _returnvalue) (`|GetArrayItem` PointArray (- PointIndex 1)) (== PointIndex 0)) (`|GetArrayItem` PointArray PointIndex) (`KismetMathLibrary.SelectVector` (`|GetArrayItem` PointArray) (`|GetArrayItem` PointArray (+ PointIndex 1)) (== PointIndex _returnvalue))))

(fn `GetNearVector`
  (params (A :type "Vector Structure") (B :type "Vector Structure") (C :type "Vector Structure"))
  (returns (BackwardVector :type "Vector Structure") (ForwardVector :type "Vector Structure"))
  (return (`KismetMathLibrary.Normal` (- A B)) (`KismetMathLibrary.Normal` (- C B))))

(fn `GetPointsFromSpline`
  (params (TargetSpline :type "SplineComponent Object Reference") (CoordinateSpace :type "ESplineCoordinateSpace Enum" :default "Local"))
  (returns (Points :type "Array of Vector Structure"))
  (locals (PointList :type "Array of Vector Structure"))
  (`KismetArrayLibrary.Array_Clear` (`local.PointList`))
  (for _index (range (`SplineComponent.GetNumberOfSplinePoints` TargetSpline))
    (`KismetArrayLibrary.Array_Add` (`local.PointList`) (`SplineComponent.GetLocationAtSplinePoint` (`local.TargetSpline`) _index (`local.CoordinateSpace`))))
  (return (`local.PointList`)))

(fn `MeshSpawner`
  (params (MeshArray :type "Array of Transform Structure") (TargetMesh :type "StaticMesh Object Reference") (SuitFloorHeight :type Boolean :default true) (FloorHeight :type "Float (double-precision)" :default 300.0) (ResetMaterial :type Boolean) (TargetMaterial :type "MaterialInterface Object Reference") (Transform :type "Transform Structure"))
  (bind (_long _width _height _alongx) (`self.GetMeshSize` TargetMesh))
  (for _array_element MeshArray
    (bind _returnvalue (`AddComponent|NODE_AddStaticMeshComponent-0` :`RelativeTransform` (`KismetMathLibrary.ComposeTransforms` (`KismetMathLibrary.MakeTransform` (`KismetMathLibrary.SelectVector` (`KismetMathLibrary.MakeVector` (.x (.location Transform)) (.y (.location Transform)) (.z (.location Transform))) (`KismetMathLibrary.MakeVector` (.y (.location Transform)) (.x (.location Transform)) (.z (.location Transform))) _alongx) (.rotation Transform) (.scale Transform)) (`KismetMathLibrary.ComposeTransforms` (`KismetMathLibrary.MakeTransform` (0.0 0.0 0.0) (`KismetMathLibrary.MakeRotator` 0.0 0.0 (`KismetMathLibrary.SelectFloat` 0.0 90.0 _alongx))) (`KismetMathLibrary.MakeTransform` (.location _array_element) (.rotation _array_element) (`KismetMathLibrary.MakeVector` (.x (.scale _array_element)) (.y (.scale _array_element)) (`KismetMathLibrary.SelectFloat` (* (.z (.scale _array_element)) (/ FloorHeight _height)) (.z (.scale _array_element)) SuitFloorHeight)))))))
    (`StaticMeshComponent.SetStaticMesh` _returnvalue TargetMesh)
    (if ResetMaterial
      (`PrimitiveComponent.SetMaterial` _returnvalue 0 TargetMaterial))))

(fn `PointLocation`
  (params (PointArray :type "Array of Transform Structure"))
  (returns (LocationArray :type "Array of Vector Structure"))
  (locals (PointArray_Var :type "Array of Vector Structure"))
  (`KismetArrayLibrary.Array_Clear` (`local.PointArray_Var`))
  (for _array_element PointArray
    (`KismetArrayLibrary.Array_Add` (`local.PointArray_Var`) (.location _array_element)))
  (return (`local.PointArray_Var`)))

(fn `PolygonMeshSpawner`
  (params (PointArray :type "Array of Vector Structure") (Thickness :type "Float (double-precision)") (OffsetZ :type "Float (double-precision)") (Shrink :type "Float (single-precision)") (MaterialOverwrite :type "MaterialInterface Object Reference"))
  (returns (`Target Mesh` :type "DynamicMesh Object Reference"))
  (locals (PolygonVertices :type "Array of Vector2D Structure"))
  (`KismetArrayLibrary.Array_Clear` (`local.PolygonVertices`))
  (for _array_element (`self.PolygonShrink` PointArray Shrink)
    (`KismetArrayLibrary.Array_Add` (`local.PolygonVertices`) (`KismetMathLibrary.MakeVector2D` (.x _array_element) (.y _array_element))))
  (bind _returnvalue (`AddComponent|NODE_AddDynamicMeshComponent-2` :`RelativeTransform` (`KismetMathLibrary.MakeTransform` (`KismetMathLibrary.MakeVector` 0.0 0.0 OffsetZ))))
  (`BaseDynamicMeshComponent.SetOverrideRenderMaterial` _returnvalue MaterialOverwrite)
  (bind _returnvalue_2 (`BaseDynamicMeshComponent.GetDynamicMesh` _returnvalue))
  (bind _returnvalue_3 (`GeometryScriptLibrary_MeshPrimitiveFunctions.AppendTriangulatedPolygon` _returnvalue_2 (struct) (struct) (`local.PolygonVertices`) true null))
  (bind _returnvalue_4 (`GeometryScriptLibrary_MeshModelingFunctions.ApplyMeshLinearExtrudeFaces` _returnvalue_3 (make `GeometryScriptMeshLinearExtrudeOptions` Thickness) (struct) null))
  (return _returnvalue_4))

(fn `PolygonPartitioningA`
  (params (InPolygon :type "Array of Vector Structure") (Obliquity :type "Float (double-precision)" :default 0.1) (SeamWidth :type "Float (double-precision)"))
  (returns (OutPolygonA :type "Array of Vector Structure") (OutPolygonB :type "Array of Vector Structure") (CutPointA :type "Vector Structure") (CutPointB :type "Vector Structure"))
  (locals (InPolygon_Var :type "Array of Vector Structure") (OutPolygonA_Var :type "Array of Vector Structure") (OutPolygonB_Var :type "Array of Vector Structure") (CutPointA_Var :type "Vector Structure" :default (0.0 0.0 0.0)) (CutPointB_Var :type "Vector Structure" :default (0.0 0.0 0.0)) (LongestEdge :type Integer :default 0) (RangeA :type "Float (double-precision)" :default 0.0) (RangeB :type "Float (double-precision)" :default 0.0) (SeamWidth_Var :type "Float (double-precision)"))
  (bind _returnvalue (+ 0.5 Obliquity))
  (bind _returnvalue_2 (- 0.5 Obliquity))
  (bind _outpolygona_var (`local.OutPolygonA_Var`))
  (bind _outpolygonb_var (`local.OutPolygonB_Var`))
  (bind _longestedge (`local.LongestEdge`))
  (`|ExecutionSequence`
    (:`then_0`
      (bind _output_get (set `local.InPolygon_Var` InPolygon))
      (set `local.LongestEdge` (`self.GetLongestEdge` _output_get))
      (set `local.RangeA` (`KismetMathLibrary.RandomFloatInRange` _returnvalue_2 _returnvalue))
      (set `local.RangeB` (`KismetMathLibrary.RandomFloatInRange` _returnvalue_2 _returnvalue))
      (set `local.SeamWidth_Var` SeamWidth))
    (:`then_1`
      (`KismetArrayLibrary.Array_Add` _outpolygona_var (`|GetArrayItem` (`local.InPolygon_Var`) (`local.LongestEdge`)))
      (`KismetArrayLibrary.Array_Add` _outpolygona_var)
      (`KismetArrayLibrary.Array_Add` _outpolygona_var)
      (`KismetArrayLibrary.Array_Add` _outpolygona_var))
    (:`then_2`
      (`KismetArrayLibrary.Array_Add` _outpolygonb_var (`|GetArrayItem` (`local.InPolygon_Var`) (`KismetMathLibrary.SelectInt` (- _longestedge 2) (+ _longestedge 2) (>= _longestedge 2))))
      (`KismetArrayLibrary.Array_Add` _outpolygonb_var)
      (`KismetArrayLibrary.Array_Add` _outpolygonb_var)
      (`KismetArrayLibrary.Array_Add` _outpolygonb_var))
    (:`then_3`
      (set `local.CutPointA_Var` (0.0 0.0 0.0))
      (set `local.CutPointB_Var` (0.0 0.0 0.0)))
    (:`then_4`
      (return (`local.OutPolygonA_Var`) (`local.OutPolygonB_Var`) (`local.CutPointA_Var`) (`local.CutPointB_Var`)))))

(fn `PolygonSampler`
  (params (CornerArray :type "Array of Vector Structure") (SpecialEdge :type "Array of Integer") (Unit_Mesh :type "StaticMesh Object Reference"))
  (returns (PointArray :type "Array of Transform Structure"))
  (locals (PointArray_Var :type "Array of Transform Structure"))
  (bind (_lastpointlocation _currentpointlocation _nextpointlocation) (`self.GetNearPoints` CornerArray))
  (`KismetArrayLibrary.Array_Clear` (`local.PointArray_Var`))
  (for (_ _array_index) CornerArray
    (if (not (`KismetArrayLibrary.Array_Contains` SpecialEdge _array_index))
      (bind _pointarray (`self.EdgeSampler` _currentpointlocation _nextpointlocation Unit_Mesh))
      (`KismetArrayLibrary.Array_Append` (`local.PointArray_Var`) _pointarray)))
  (return (`local.PointArray_Var`)))

(fn `PolygonShrink`
  (params (PointArray :type "Array of Vector Structure") (Shrink :type "Float (single-precision)"))
  (returns (OutPointArray :type "Array of Vector Structure"))
  (locals (TargetPointArray :type "Array of Vector Structure"))
  (`KismetArrayLibrary.Array_Clear` (`local.TargetPointArray`))
  (for (_ _array_index) PointArray
    (bind (_lastpointlocation _currentpointlocation _nextpointlocation) (`self.GetNearPoints` PointArray _array_index))
    (bind _returnvalue (`KismetMathLibrary.Normal` (- _lastpointlocation _currentpointlocation)))
    (bind _returnvalue_2 (`KismetMathLibrary.Normal` (- _nextpointlocation _currentpointlocation)))
    (bind (_returnvalue_x _returnvalue_y _returnvalue_z) (`KismetMathLibrary.BreakVector` (`KismetMathLibrary.Cross_VectorVector` _returnvalue _returnvalue_2)))
    (`KismetArrayLibrary.Array_Add` (`local.TargetPointArray`) (+ (* (`KismetMathLibrary.Normal` (+ _returnvalue _returnvalue_2)) (`KismetMathLibrary.SelectFloat` -1.0 1.0 (> _returnvalue_z 0.0)) Shrink) _currentpointlocation)))
  (return (`local.TargetPointArray`)))

(fn `SplineMeshSpowner`
  (params (Spline :type "SplineComponent Object Reference") (SplineMesh :type "StaticMesh Object Reference") (SplineMaterial :type "MaterialInstance Object Reference") (StartDistance :type "Float (double-precision)") (EndDistance :type "Float (double-precision)" :default 3000.0) (ForwardAxis :type "ESplineMeshAxis Enum" :default "X") (UnitScale :type "Vector Structure" :default (1.0 1.0 1.0)) (Te :type "Float (double-precision)") (Roll :type "Float (double-precision)") (OffsetY :type "Float (double-precision)") (OffsetZ :type "Float (double-precision)") (Reversed :type Boolean) (ByZone :type Boolean) (Spawn :type Boolean :default true) (CoordinateSpace :type "ESplineCoordinateSpace Enum" :default "Local"))
  (locals (MeshLength :type "Float (double-precision)") (SplingLength :type "Float (single-precision)") (DistanceA :type "Float (double-precision)") (DistanceB :type "Float (double-precision)") (Spline_Var :type "SplineComponent Object Reference") (SplineMeshComponent :type "SplineMeshComponent Object Reference"))
  (bind _unitscale_x (`KismetMathLibrary.BreakVector` (`local.UnitScale`)))
  (bind _spline (`local.Spline`))
  (bind _coordinatespace (`local.CoordinateSpace`))
  (bind _reversed (`local.Reversed`))
  (bind (_unitscale_x_2 _unitscale_y _unitscale_z) (`KismetMathLibrary.BreakVector` (`local.UnitScale`)))
  (bind _offsetz (`local.OffsetZ`))
  (bind _returnvalue (`KismetMathLibrary.SelectFloat` -1.0 1.0 (`local.Reversed`)))
  (bind _returnvalue_2 (`SplineComponent.GetSplineLength` (`local.Spline`)))
  (bind _returnvalue_3 (/ (`local.MeshLength`) 2.0))
  (bind (_min _max) (break `Box` (`StaticMesh.GetBoundingBox` (`local.SplineMesh`))))
  (bind (_long _count) (`self.Average` (`local.SplingLength`) (- (`local.MeshLength`) 0.0)))
  (bind _returnvalue_4 (+ (select `ESplineMeshAxis` (`local.ForwardAxis`) :`Y` -90.0) (`local.Roll`)))
  (bind _returnvalue_5 (* (`local.OffsetY`) (`KismetMathLibrary.SelectFloat` -1.0 1.0 (`local.Reversed`))))
  (bind (_returnvalue_x _returnvalue_y _returnvalue_z) (`KismetMathLibrary.BreakVector` (- _min _max)))
  (bind _returnvalue_6 (/ (`local.SplingLength`) _count))
  (if (`local.Spawn`)
    (set `local.Spline_Var` Spline)
    (set `local.MeshLength` (* (select `ESplineMeshAxis` (`local.ForwardAxis`) :`X` (`KismetMathLibrary.Abs` _returnvalue_x) :`Y` (`KismetMathLibrary.Abs` _returnvalue_y) :`Z` (`KismetMathLibrary.Abs` _returnvalue_z)) _unitscale_x))
    (set `local.SplingLength` (`KismetMathLibrary.SelectFloat` (`KismetMathLibrary.FMin` (`KismetMathLibrary.Abs` (- (`local.StartDistance`) (`local.EndDistance`))) _returnvalue_2) _returnvalue_2 (`local.ByZone`)))
    (for _index (range _count)
      (`|ExecutionSequence`
        (:`then_0`
          (bind _returnvalue_7 (* _index _returnvalue_6))
          (bind _returnvalue_8 (+ _returnvalue_7 _returnvalue_6 0.0))
          (bind _returnvalue_9 (`KismetMathLibrary.SelectFloat` _returnvalue_8 _returnvalue_7 _reversed))
          (set `local.DistanceA` (`KismetMathLibrary.SelectFloat` (+ (`local.StartDistance`) _returnvalue_9) _returnvalue_9 (`local.ByZone`)))
          (bind _returnvalue_10 (`KismetMathLibrary.SelectFloat` _returnvalue_7 _returnvalue_8 _reversed))
          (set `local.DistanceB` (`KismetMathLibrary.SelectFloat` (+ (`local.StartDistance`) _returnvalue_10) _returnvalue_10 (`local.ByZone`))))
        (:`then_1`
          (bind _returnvalue_11 (`AddComponent|NODE_AddSplineMeshComponent-1`))
          (set `local.SplineMeshComponent` _returnvalue_11)
          (`SplineMeshComponent.SetForwardAxis` (`local.SplineMeshComponent`) (`local.ForwardAxis`) true)
          (`StaticMeshComponent.SetStaticMesh` (`local.SplineMeshComponent`) (`local.SplineMesh`))
          (`PrimitiveComponent.SetCollisionEnabled` (`local.SplineMeshComponent`) "QueryAndPhysics"))
        (:`then_2`
          (`SplineMeshComponent.SetStartAndEnd` (`local.SplineMeshComponent`) (`SplineComponent.GetLocationAtDistanceAlongSpline` _spline (`local.DistanceA`) _coordinatespace) (* (`SplineComponent.GetDirectionAtDistanceAlongSpline` _spline (`local.DistanceA`) _coordinatespace) _returnvalue_3 (`KismetMathLibrary.SelectFloat` -1.0 1.0 (`local.Reversed`))) (`SplineComponent.GetLocationAtDistanceAlongSpline` _spline (`local.DistanceB`) _coordinatespace) (* (`SplineComponent.GetDirectionAtDistanceAlongSpline` _spline (`local.DistanceB`) _coordinatespace) _returnvalue_3 (`KismetMathLibrary.SelectFloat` -1.0 1.0 (`local.Reversed`))) true)
          (`SplineMeshComponent.SetStartScale` (`local.SplineMeshComponent`) (`KismetMathLibrary.MakeVector2D` _unitscale_y _unitscale_z) true)
          (`SplineMeshComponent.SetEndScale` (`local.SplineMeshComponent`) (`KismetMathLibrary.MakeVector2D` _unitscale_y _unitscale_z) true)
          (`SplineMeshComponent.SetStartRoll` (`local.SplineMeshComponent`) (* (`KismetMathLibrary.DegreesToRadians` (+ (`SplineComponent.GetRollAtDistanceAlongSpline` _spline (`local.DistanceA`) _coordinatespace) _returnvalue_4)) _returnvalue) true)
          (`SplineMeshComponent.SetEndRoll` (`local.SplineMeshComponent`) (* (`KismetMathLibrary.DegreesToRadians` (+ (`SplineComponent.GetRollAtDistanceAlongSpline` _spline (`local.DistanceB`) _coordinatespace) _returnvalue_4)) _returnvalue) true)
          (`SplineMeshComponent.SetStartOffset` (`local.SplineMeshComponent`) (`KismetMathLibrary.MakeVector2D` _returnvalue_5 _offsetz) true)
          (`SplineMeshComponent.SetEndOffset` (`local.SplineMeshComponent`) (`KismetMathLibrary.MakeVector2D` _returnvalue_5 _offsetz) true))))))

(fn `SplineShrink`
  (params (SplineA :type "SplineComponent Object Reference") (SplineB :type "SplineComponent Object Reference") (Shrink :type "Float (double-precision)"))
  (locals (SplinePointsA :type "Array of Vector Structure") (SplinePointsB :type "Array of Vector Structure"))
  (bind _splinea (`local.SplineA`))
  (`|ExecutionSequence`
    (:`then_0`
      (`KismetArrayLibrary.Array_Clear` (`local.SplinePointsA`))
      (for _index (range (+ (`.ReturnValue` (`KismetMathLibrary.FMod` (`SplineComponent.GetSplineLength` (`local.SplineA`)) 500.0)) 1))
        (bind _returnvalue (* _index 500))
        (`KismetArrayLibrary.Array_Add` (`local.SplinePointsA`) (+ (`SplineComponent.GetLocationAtDistanceAlongSpline` _splinea _returnvalue "Local") (* (`SplineComponent.GetRightVectorAtDistanceAlongSpline` _splinea _returnvalue "Local") (`local.Shrink`))))))
    (:`then_2`
      (`SplineComponent.SetSplinePoints` (`local.SplineB`) (`local.SplinePointsA`) "Local" true)
      (`SplineComponent.SetClosedLoop` (`local.SplineB`) true true))))

(fn `SplineThingsSpowner`
  (params (Spline :type "SplineComponent Object Reference") (Mesh :type "StaticMesh Object Reference") (StartDistance :type "Float (double-precision)") (EndDistance :type "Float (double-precision)" :default 3000.0) (Spacing :type "Float (double-precision)" :default 500.0) (Offset :type "Vector Structure") (Scale :type "Vector Structure" :default (1.0 1.0 1.0)) (Rotation :type "Rotator Structure") (ByZone :type Boolean) (AlongSplineDir :type Boolean))
  (bind _returnvalue (`SplineComponent.GetSplineLength` Spline))
  (bind _spline (`local.Spline`))
  (bind (_long _count) (`self.Average` (`KismetMathLibrary.SelectFloat` (`KismetMathLibrary.FMin` _returnvalue (`KismetMathLibrary.Abs` (- (`local.StartDistance`) (`local.EndDistance`)))) _returnvalue (`local.ByZone`)) Spacing))
  (for _index (range (+ _count 1))
    (bind _returnvalue_2 (* _index _long))
    (bind _returnvalue_3 (`KismetMathLibrary.SelectFloat` (+ _returnvalue_2 (`local.StartDistance`)) _returnvalue_2 (`local.ByZone`)))
    (bind _returnvalue_4 (`AddComponent|NODE_AddStaticMeshComponent-1` :`RelativeTransform` (`KismetMathLibrary.ComposeTransforms` (`KismetMathLibrary.MakeTransform` (`local.Offset`) (`local.Rotation`) (`local.Scale`)) (`KismetMathLibrary.MakeTransform` (`SplineComponent.GetLocationAtDistanceAlongSpline` _spline _returnvalue_3 "Local") (`KismetMathLibrary.SelectRotator` (`SplineComponent.GetRotationAtDistanceAlongSpline` _spline _returnvalue_3 "Local") (struct) (`local.AlongSplineDir`))))))
    (`StaticMeshComponent.SetStaticMesh` _returnvalue_4 (`local.Mesh`))))

(fn `UserConstructionScript`)